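; Player controller Blueprint that holds the player's resource stores of power, wood, coal and oil in a resource-management setup.
; Each resource has its own custom check event that uses a Sequence to clamp the amount between zero and that resource's maximum.
; BeginPlay and Tick are empty, and nothing in this graph changes the amounts or calls the checks.
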(event Custom|CheckPowerStorage
  ;[1 1 1] Makes power not go over max or below zero
  (Utilities|FlowControl|Sequence
    (:then_0
      (if (>= (Variables|Power|GetPowerAmount) (Variables|Power|GetPowerStorageMax))
        (Variables|Power|SetPowerAmount (Variables|Power|GetPowerStorageMax))))
    (:then_1
      (if (<= (Variables|Power|GetPowerAmount) 0.0)
        (Variables|Power|SetPowerAmount 0.0)))))

(event Custom|CheckWoodStorage
  ;[1 0.6723 0.4679] Stop Wood from going past Max
  (Utilities|FlowControl|Sequence
    (:then_0
      (if (>= (Variables|Wood|GetWoodAmount) (Variables|Wood|GetMaxWoodAmount))
        (Variables|Wood|SetWoodAmount (Variables|Wood|GetMaxWoodAmount))))
    (:then_1
      (if (<= (Variables|Wood|GetWoodAmount) 0.0)
        (Variables|Wood|SetWoodAmount 0.0)))))

(event Custom|CheckCoalStorage
  ;[0.08674 0.06999 0.1875] Stop Coal from going past Max
  (Utilities|FlowControl|Sequence
    (:then_0
      (if (>= (Variables|Coal|GetCoalAmount) (Variables|Coal|GetMaxCoalAmount))
        (Variables|Coal|SetCoalAmount (Variables|Coal|GetMaxCoalAmount))))
    (:then_1
      (if (<= (Variables|Coal|GetCoalAmount) 0.0)
        (Variables|Coal|SetCoalAmount 0.0)))))

(event Custom|CheckOilStorage
  ;[0 0 0] Stop Oil from going past Max
  (Utilities|FlowControl|Sequence
    (:then_0
      (if (>= (Variables|Oil|GetOilAmount) (Variables|Oil|GetMaxOilAmount))
        (Variables|Oil|SetOilAmount (Variables|Oil|GetMaxOilAmount))))
    (:then_1
      (if (<= (Variables|Oil|GetOilAmount) 0.0)
        (Variables|Oil|SetOilAmount 0.0)))))

(event EventBeginPlay)

(event EventTick
  (params (DeltaSeconds :type Float%20%28single-precision%29)))

(fn ConstructionScript)